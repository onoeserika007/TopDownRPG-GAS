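; Electrocute gameplay ability: a channeled lightning beam fired at the target under the mouse, chaining to additional targets when it hits a combat actor.
; A montage event locks movement, adds looping shock cues and starts a timer that commits cost and deals damage each tick.
; Input release, failed cost or primary target death ends it, applying final damage and clearing cues, with cooldown depending on hold time.
; Additional targets drop out individually on death.
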(event Custom|DamageAndCost
  (bind _returnvalue (Ability|CommitAbilityCost false))
  (if _returnvalue
    (CallFunction|ApplyDamage)
    (else
      (CallFunction|PreEndAbility)
      ;[1 1 1] This will force to end, waitingForRelease will no longer work
      (Ability|EndAbility))))

(event Ability|EventActivateAbility
  (if (Utilities|DoesObjectImplementInterface (Ability|GetAvatarActorfromActorInfo) "/Script/Aura.CombatInterface")
    (bind _datahandle (|TargetDataUnderMouse)
      (:ValidData
        (Class|AuraBeamSpell|StoreMouseDataInfo (Ability|TargetData|GetHitResultfromTargetData _datahandle))
        (Class|AuraBeamSpell|StoreOwnerVariables)
        (Utilities|FlowControl|Sequence
          (:then_0
            (Variables|/Script/Engine.PlayerController|SetbShowMouseCursor (Variables|Default|GetOwnerPlayerController) false)
            (Class|CombatInterface|SetFacingTarget(Message) (Ability|GetAvatarActorfromActorInfo) (Variables|Default|GetMouseHitLocation))
            ;[1 1 1] Burst Sound
            (GameplayCue|ExecuteGameplayCue :GameplayCueTag "(TagName=\"GameplayCue.ShockBurst\")")
            (|PlayMontageandWaitProxy "None" (Variables|Default|GetElectrocuteMontage) 1.0 "None" true 1.0 0.0
              (:then
                (Ability|Tasks|WaitGameplayEvent "(TagName=\"Event.Montage.Electrocute\")" 0 true
                  (:EventReceived
                    (Pawn|Components|CharacterMovement|SetMovementMode (Variables|/Script/Engine.Character|GetCharacterMovement (Variables|Default|GetOwnerCharacter)) "MOVE_None" 0)
                    (Class|CombatInterface|SetinShockLoop(Message) (Ability|GetAvatarActorfromActorInfo) true)
                    (CallFunction|SpawnElectricBeam)
                    (bind _returnvalue (Utilities|Time|SetTimerbyEvent (delegate Custom|DamageAndCost) (Variables|Default|GetDamageDeltaTime) true))
                    (Variables|Default|SetDamageAndCostTimer _returnvalue))))))
          (:then_1
            (bind _timeheld (Ability|Tasks|WaitInputRelease true)
              (:OnRelease
                (Variables|Default|SetTime%20Held _timeheld)
                (CallFunction|PreEndAbility)
                (Ability|EndAbility)))))))
    (else
      (Ability|EndAbility))))

(event Ability|EventOnEndAbility
  (params (bWasCancelled :type Boolean)))

(event EventAdditionalActorDied
  (params (DeadActor :type Actor%20Object%20Reference))
  (CallFunction|RemoveShockLoopCuefromAdditionalTarget DeadActor)
  (Class|AuraBeamSpell|UnbindAllTargetDiedCallback DeadActor)
  (Utilities|Array|RemoveItem (Variables|Default|GetAdditionalTargets) DeadActor))

(event EventPrimaryTargetDied
  (params (DeadActor :type Actor%20Object%20Reference))
  (CallFunction|PreEndAbility)
  (Ability|EndAbility))

(fn SpawnElectricBeam
  (Class|AuraBeamSpell|TraceFirstTarget (Variables|Default|GetMouseHitLocation))
  (bind _returnvalue (Class|CombatInterface|GetWeapon(Message) (Ability|GetAvatarActorfromActorInfo)))
  (LocalVariables|SetWeaponMesh _returnvalue)
  ;[1 1 1] Is MouseHitActor an Enemy?
  (Variables|Default|SetFirstTargetCueParams (Ability|GameplayCue|MakeGameplayCueParameters :Location (Variables|Default|GetMouseHitLocation) :SourceObject (Variables|Default|GetMouseHitActor) :TargetAttachComponent _returnvalue))
  (if (Utilities|DoesObjectImplementInterface (Variables|Default|GetMouseHitActor) "/Script/Aura.CombatInterface")
    (Variables|Default|SetCueTarget (Variables|Default|GetMouseHitActor))
    (Class|AuraBeamSpell|BindPrimaryTargetDiedCallback (Variables|Default|GetMouseHitActor))
    (Class|CombatInterface|SetIsBeingShocked(Message) (Variables|Default|GetMouseHitActor) true)
    (bind _outadditionaltargets (Class|AuraBeamSpell|StoreAdditionalTargets))
    (bind _output_get (Variables|Default|SetAdditionalTargets _outadditionaltargets))
    (for _array_element _output_get
      (CallFunction|AddShockLoopCuetoAdditionalTarget _array_element)
      (Class|AuraBeamSpell|BindAdditionalTargetDiedCallback _array_element)
      (Class|CombatInterface|SetIsBeingShocked(Message) _array_element true))
    (else
      (Variables|Default|SetCueTarget (Variables|Default|GetMouseHitActor))))
  (GameplayCue|AddGameplayCueOnActor(Looping) (Variables|Default|GetCueTarget) "(TagName=\"GameplayCue.ShockLoop\")" (Variables|Default|GetFirstTargetCueParams)))

(fn AddShockLoopCuetoAdditionalTarget
  (params (Additional%20Target :type Actor%20Object%20Reference))
  (bind _output_get (LocalVariables|SetTargetActor Additional%20Target))
  (Utilities|Map|Add (Variables|Default|GetAdditionalActorsToCueParams) _output_get (Ability|GameplayCue|MakeGameplayCueParameters :Location (Transformation|GetActorLocation (LocalVariables|GetTargetActor)) :SourceObject (LocalVariables|GetTargetActor) :TargetAttachComponent (Variables|/Script/Engine.Actor|GetRootComponent (Variables|Default|GetMouseHitActor))))
  (GameplayCue|AddGameplayCueOnActor(Looping) (LocalVariables|GetTargetActor) "(TagName=\"GameplayCue.ShockLoop\")" (Ability|GameplayCue|MakeGameplayCueParameters :Location (Transformation|GetActorLocation (LocalVariables|GetTargetActor)) :SourceObject (LocalVariables|GetTargetActor) :TargetAttachComponent (Variables|/Script/Engine.Actor|GetRootComponent (Variables|Default|GetMouseHitActor)))))

(fn RemoveShockLoopCuefromAdditionalTarget
  (params (Target%20Actor :type Actor%20Object%20Reference))
  (bind _additionalactorstocueparams (Variables|Default|GetAdditionalActorsToCueParams))
  (bind (_value _returnvalue) (Utilities|Map|Find _additionalactorstocueparams Target%20Actor))
  (if _returnvalue
    (GameplayCue|RemoveGameplayCueOnActor(Looping) Target%20Actor "(TagName=\"GameplayCue.ShockLoop\")" _value)))

(fn PreEndAbility
  (if (>= (Variables|Default|GetTime%20Held) (Variables|Default|GetMinSpellTime))
    (Ability|CommitAbilityCooldown false))
  (Variables|/Script/Engine.PlayerController|SetbShowMouseCursor (Variables|Default|GetOwnerPlayerController) true)
  (Class|CombatInterface|SetinShockLoop(Message) (Ability|GetAvatarActorfromActorInfo) false)
  (GameplayCue|RemoveGameplayCueOnActor(Looping) (Variables|Default|GetCueTarget) "(TagName=\"GameplayCue.ShockLoop\")" (Variables|Default|GetFirstTargetCueParams))
  (Class|AuraBeamSpell|UnbindAllTargetDiedCallback (Variables|Default|GetCueTarget))
  (if (Utilities|DoesObjectImplementInterface (Variables|Default|GetCueTarget) "/Script/Aura.CombatInterface")
    (Class|CombatInterface|SetIsBeingShocked(Message) (Variables|Default|GetCueTarget) false)
    (Class|AuraAbilitySystemLibrary|ApplyDamageEffect (Class|AuraDamageGameplayAbility|MakeDamageEffectParamsfromClassDefaults (Variables|Default|GetCueTarget) "0, 0, 0" false "0, 0, 0" false "0, 0, 0" false 0.0)))
  (for _array_element (Variables|Default|GetAdditionalTargets)
    (CallFunction|RemoveShockLoopCuefromAdditionalTarget _array_element)
    (Class|AuraBeamSpell|UnbindAllTargetDiedCallback _array_element)
    (if (Utilities|DoesObjectImplementInterface _array_element "/Script/Aura.CombatInterface")
      (Class|AuraAbilitySystemLibrary|ApplyDamageEffect (Class|AuraDamageGameplayAbility|MakeDamageEffectParamsfromClassDefaults _array_element "0, 0, 0" false "0, 0, 0" false "0, 0, 0" false 0.0))
      (Class|CombatInterface|SetIsBeingShocked(Message) _array_element false)))
  (Utilities|Time|ClearandInvalidateTimerbyHandle (Variables|Default|GetDamageAndCostTimer))
  (Pawn|Components|CharacterMovement|SetMovementMode (Variables|/Script/Engine.Character|GetCharacterMovement (Variables|Default|GetOwnerCharacter)) "MOVE_Walking" 0)
  (Utilities|Map|Clear (Variables|Default|GetAdditionalActorsToCueParams))
  (Utilities|Array|Clear (Variables|Default|GetAdditionalTargets))
  (Variables|Default|SetMouseHitActor 0)
  (Variables|Default|SetCueTarget 0))

(fn ApplyDamage
  (CallFunction|ApplyDamageSingleTarget (Variables|Default|GetMouseHitActor))
  (for _array_element (Variables|Default|GetAdditionalTargets)
    (CallFunction|ApplyDamageSingleTarget _array_element)))

(fn ApplyDamageSingleTarget
  (params (Actor :type Actor%20Object%20Reference))
  (bind _returnvalue (Class|AuraDamageGameplayAbility|MakeDamageEffectParamsfromClassDefaults Actor "0, 0, 0" false "0, 0, 0" false "0, 0, 0" false 0.0))
  (bind (_worldcontextobject _damagegameplayeffectclass _sourceabilitysystemcomponent _targetabilitysystemcomponent _basedamage _abilitylevel _damagetype _debuffchance _debuffdamage _debuffduration _debufffrequency _deathimpulsemagnitude _deathimpulse _knockbackforcemagnitude _knockbackchance _knockbackforce) (Utilities|Struct|BreakDamageEffectParams _returnvalue))
  (Utilities|IsValid (Ability|GetAbilitySystemComponent Actor)
    (:Is%20Valid
      (Class|AuraAbilitySystemLibrary|ApplyDamageEffect (Utilities|Struct|MakeDamageEffectParams _worldcontextobject _damagegameplayeffectclass _sourceabilitysystemcomponent _targetabilitysystemcomponent _basedamage _abilitylevel _damagetype 0.0 _debuffdamage _debuffduration _debufffrequency _deathimpulsemagnitude _deathimpulse _knockbackforcemagnitude _knockbackchance _knockbackforce)))))