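; Arcane Shards ability that shows a magic circle, then on an input press takes the point under the mouse and pays the cost.
; A temporary BP_PointCollection supplies ground points at random yaw, one per ability level up to a cap.
; After a montage event, a looping timer calls SpawnShard at each point, firing a gameplay cue and radial damage with outward knockback.
; Cooldown commits after the last shard; debug spheres and print remain.
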(event Custom|PreEndAbility
  (Ability|CommitAbilityCooldown false)
  (Variables|Default|SetCount 0)
  (Utilities|FlowControl|Delay 0.0)
  (Utilities|Array|Clear (Variables|Default|GetGroudPoints))
  (bind _pointcollection (Variables|Default|GetPointCollection)
    (:then
      (Actor|DestroyActor _pointcollection))
    (:else)))

(event Ability|EventActivateAbility
  (Utilities|FlowControl|Sequence
    (:then_0
      (Class|PlayerInterface|ShowMagicCircle(Message) (Ability|GetAvatarActorfromActorInfo) 0)
      (Variables|Default|SetNumPoints (Math|Integer|Min(Integer) (Ability|GetAbilityLevel) (Variables|Default|GetMaxNumShards))))
    (:then_1
      (Ability|Tasks|WaitInputPress false
        (:OnPress
          (Utilities|FlowControl|Sequence
            (:then_0
              (bind _datahandle (|TargetDataUnderMouse)
                (:ValidData
                  (Variables|Default|SetMouseHitLocation (.ImpactPoint (Collision|BreakHitResult (Ability|TargetData|GetHitResultfromTargetData _datahandle))))
                  (bind _returnvalue (Game|SpawnActorfromClass "/Game/Blueprints/AbilitySystem/GameplayAbilities/Aura/Arcane/ArcaneShards/BP_PointCollection.BP_PointCollection_C" (Math|Transform|MakeTransform (Variables|Default|GetMouseHitLocation) "0, 0, 0" "1.000000,1.000000,1.000000") "AlwaysSpawn" "MultiplyWithRoot" 0 0))
                  (Variables|Default|SetPointCollection _returnvalue)
                  (Variables|Default|SetGroudPoints (Class|PointCollection|GetGroundPoints _returnvalue (Variables|Default|GetMouseHitLocation) (Variables|Default|GetNumPoints) (Math|Random|RandomFloatinRange 0.0 3.6e+02)))
                  (Class|CombatInterface|SetFacingTarget(Message) (Ability|GetAvatarActorfromActorInfo) (Variables|Default|GetMouseHitLocation)))))
            (:then_1
              (bind _returnvalue_2 (Ability|CommitAbilityCost false))
              (if _returnvalue_2
                (|PlayMontageandWaitProxy "None" (Variables|Default|GetArcaneShardsMontage) 1.0 "None" true 1.0 0.0
                  (:then
                    (Ability|Tasks|WaitGameplayEvent "(TagName=\"Event.Montage.ArcaneShards\")" 0 true
                      (:EventReceived
                        (bind _returnvalue_3 (Utilities|Time|SetTimerbyEvent (EventDispatchers|CreateEvent :!event SpawnShard) (Variables|Default|GetShardSpawnDeltaTime) true))
                        (Variables|Default|SetShardSpawnTimer _returnvalue_3)
                        (CallFunction|SpawnShard)
                        (Class|PlayerInterface|HideMagicCircle(Message) (Ability|GetAvatarActorfromActorInfo))))))
                (else
                  (Class|PlayerInterface|HideMagicCircle(Message) (Ability|GetAvatarActorfromActorInfo))
                  (Ability|EndAbility))))))))))

(event Ability|EventOnEndAbility
  (params (bWasCancelled :type Boolean))
  (Development|PrintString "Arcane Shards Ended." true true "(R=1.000000,G=0.090171,B=0.103435,A=1.000000)" 5.0))

(fn SpawnShard
  (bind _returnvalue (Ability|GetAvatarActorfromActorInfo))
  (LocalVariables|SetShardSpawnLocation (Transformation|GetWorldLocation (Utilities|Array|Get(acopy) (Variables|Default|GetGroudPoints) (Variables|Default|GetCount))))
  (Utilities|FlowControl|Sequence
    (:then_0
      (Rendering|Debug|DrawDebugSphere (LocalVariables|GetShardSpawnLocation) (Variables|Default|GetRadialDamageInnerRadius) 12 "(R=1.000000,G=0.821264,B=0.000000,A=1.000000)" 1e+01)
      (Rendering|Debug|DrawDebugSphere (LocalVariables|GetShardSpawnLocation) (Variables|Default|GetRadialDamageOuterRadius) 12 "(R=0.000000,G=0.126143,B=1.000000,A=1.000000)" 1e+01)
      (Class|GameplayAbility|ExecuteGameplayCuewithParams "(TagName=\"GameplayCue.ArcaneShards\")" (Ability|GameplayCue|MakeGameplayCueParameters :Location (LocalVariables|GetShardSpawnLocation)))
      (bind _outoverlappingactors (Class|AuraAbilitySystemLibrary|GetLivePlayersWithinRadius _returnvalue (Utilities|Array|MakeArray _returnvalue) (Variables|Default|GetRadialDamageOuterRadius) (LocalVariables|GetShardSpawnLocation)))
      (for _array_element _outoverlappingactors
        (Class|AuraAbilitySystemLibrary|ApplyDamageEffect (Class|AuraDamageGameplayAbility|MakeDamageEffectParamsfromClassDefaults _array_element (LocalVariables|GetShardSpawnLocation) true (Math|Vector|Normalize (- (Transformation|GetActorLocation _array_element) (LocalVariables|GetShardSpawnLocation))) true (Math|Vector|Normalize (- (Transformation|GetActorLocation _array_element) (LocalVariables|GetShardSpawnLocation))) true 45.0))))
    (:then_1
      (Math|Integer|IncrementInt (Variables|Default|GetCount)))
    (:then_2
      (if (== (Variables|Default|GetCount) (Variables|Default|GetNumPoints))
        (Utilities|Time|ClearandInvalidateTimerbyHandle (Variables|Default|GetShardSpawnTimer))
        (CallFunction|PreEndAbility)
        (Ability|EndAbility)))))