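; BP_FireBall is a boomerang-style projectile for the Aura FireBlast ability that flies out, returns and explodes.
; On authority, one timeline lerps it forward to an apex at TravelDistance, then a second moves it between that apex and ReturnToActor's live location.
; Within ExplodeDistance of that actor, it applies radial damage with impulse and knockback to nearby live players, excluding its owner, then destroys itself.
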(event EventBeginPlay)

(event Collision|EventActorBeginOverlap
  (params (OtherActor :type Actor%20Object%20Reference)))

(event EventTick
  (params (DeltaSeconds :type Float%20%28single-precision%29)))

(event EventStartOutgoingTimeline
  (bind _explosiondamageparams (Variables|Default|GetExplosionDamageParams))
  (bind _explosiondamageparams_2 (Variables|Default|GetExplosionDamageParams))
  (Networking|SwitchHasAuthority
    (:Authority
      (Variables|Default|SetInitialLocation (Transformation|GetActorLocation))
      (Variables|Default|SetApexLocation (+ (Variables|Default|GetInitialLocation) (* (Transformation|GetActorForwardVector) (Variables|Default|GetTravelDistance))))
      (bind _outgoing (Timeline|OutgoingTimeline PlayFromStart)
        (:Update
          (Transformation|SetActorLocation (Math|Vector|Lerp(Vector) (Variables|Default|GetInitialLocation) (Variables|Default|GetApexLocation) _outgoing) false false))
        (:Finished
          (bind _returning (Timeline|ReturningTimeline PlayFromStart)
            (:Update
              (Variables|Default|SetCurrentaLocation (Math|Vector|Lerp(Vector) (Transformation|GetActorLocation (Variables|Default|GetReturnToActor)) (Variables|Default|GetApexLocation) _returning))
              (Transformation|SetActorLocation (Math|Vector|Lerp(Vector) (Transformation|GetActorLocation (Variables|Default|GetReturnToActor)) (Variables|Default|GetApexLocation) _returning) false false)
              (if (CallFunction|IsWithinRange)
                (bind _outoverlappingactors (Class|AuraAbilitySystemLibrary|GetLivePlayersWithinRadius 0 (Utilities|Array|MakeArray (Components|GetOwner)) 1e+02 (Transformation|GetActorLocation)))
                (for _array_element _outoverlappingactors
                  (Class|AuraAbilitySystemLibrary|SetRadialDamageEffectParam _explosiondamageparams_2 true 5e+01 1e+02 (Transformation|GetActorLocation))
                  (Class|AuraAbilitySystemLibrary|SetImpulseDamageEffectParam _explosiondamageparams_2 (- (Transformation|GetActorLocation _array_element) (Transformation|GetActorLocation)) (- (Transformation|GetActorLocation _array_element) (Transformation|GetActorLocation)) 1e+03 1e+03)
                  (Class|AuraAbilitySystemLibrary|SetTargetDamageEffectParam _explosiondamageparams _array_element)
                  (Class|AuraAbilitySystemLibrary|ApplyDamageEffect _explosiondamageparams))
                (Actor|DestroyActor)))))))))

(fn ConstructionScript)

(fn IsWithinRange
  (return (<= (Math|Vector|VectorLength (- (Transformation|GetActorLocation (Variables|Default|GetReturnToActor)) (Variables|Default|GetCurrentaLocation))) (Variables|Default|GetExplodeDistance))))