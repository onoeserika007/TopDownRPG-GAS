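; Firebolt projectile actor for the Aura fire ability, with on-hit effects.
; Its Sphere's query-only collision switches on shortly after BeginPlay.
; Tick compares the current and last-frame locations to detect a stalled bolt, then plays hit effects and destroys it on the authority only.
; The overlap events hold no logic in this Blueprint.
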(event OnComponentBeginOverlap(Sphere)
  (params (OverlappedComponent :type Primitive%20Component%20Object%20Reference) (OtherActor :type Actor%20Object%20Reference) (OtherComp :type Primitive%20Component%20Object%20Reference) (OtherBodyIndex :type Integer) (bFromSweep :type Boolean) (SweepResult :type Hit%20Result%20Structure%20%28by%20ref%29)))

(event EventBeginPlay
  (Utilities|FlowControl|Delay 0.05)
  (Collision|SetCollisionEnabled (Variables|Default|GetSphere) "QueryOnly"))

(event Collision|EventActorBeginOverlap
  (params (OtherActor :type Actor%20Object%20Reference)))

(event EventTick
  (params (DeltaSeconds :type Float%20%28single-precision%29))
  (Variables|Default|SetLocationLastFrame (Variables|Default|GetLocationThisFrame))
  (Variables|Default|SetLocationThisFrame (Transformation|GetActorLocation))
  (if (Utilities|Operators|EqualEqual (Variables|Default|GetLocationThisFrame) (Variables|Default|GetLocationLastFrame) 1.0)
    (Networking|SwitchHasAuthority
      (:Authority
        (Class|AuraProjectile|PlayonHitEffects)
        (Actor|DestroyActor)))))

(fn ConstructionScript)