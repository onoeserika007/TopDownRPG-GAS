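; Firebolt gameplay ability that casts homing projectiles from the weapon socket toward the target under the mouse.
; It commits with debug prints, takes the cursor hit, turns the avatar to face it and plays the cast montage.
; A montage gameplay event triggers the spawn, then a debug delay precedes EndAbility, which montage completion, interruption or cancellation also calls.
; The other functions are empty or default-value stubs.
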(event Ability|EventActivateAbility
  (bind _returnvalue (Ability|CommitAbility))
  (if _returnvalue
    (Development|PrintString "GA_FireBolt commit success" true true "(R=0.000000,G=0.660000,B=1.000000,A=1.000000)" 5.0)
    (else
      (Development|PrintString "GA_FireBolt commit Failed" true true "(R=0.000000,G=0.660000,B=1.000000,A=1.000000)" 5.0)))
  (bind _datahandle (|TargetDataUnderMouse)
    (:ValidData
      (Variables|Default|SetTargetLocation (.Location (Collision|BreakHitResult (Ability|TargetData|GetHitResultfromTargetData _datahandle))))
      (Variables|Default|SetMouseHitActor (.HitActor (Collision|BreakHitResult (Ability|TargetData|GetHitResultfromTargetData _datahandle))))
      (Class|CombatInterface|SetFacingTarget(Message) (Ability|GetAvatarActorfromActorInfo) (Variables|Default|GetTargetLocation))
      (|PlayMontageandWaitProxy "None" "/Game/Blueprints/Character/Aura/Cast_FireBolt_Montage.Cast_FireBolt_Montage" 1.0 "None" true 1.0 0.0
        (:then
          (Ability|Tasks|WaitGameplayEvent "(TagName=\"Event.Montage.FireBolt\")" 0
            (:EventReceived
              (Class|AuraFireBolt|SpawnProjectiles (Variables|Default|GetTargetLocation) (GameplayTags|MakeLiteralGameplayTag "(TagName=\"CombatSocket.Weapon\")") false 0.0 (Variables|Default|GetMouseHitActor))
              (Utilities|FlowControl|Delay 5.0)
              (Development|PrintText "Timer is up!")
              (Ability|EndAbility))))
        (:OnCompleted
          (Ability|EndAbility :!label _label))
        (:OnInterrupted
          (goto _label))
        (:OnCancelled
          (goto _label))))))

(event Ability|EventOnEndAbility
  (params (bWasCancelled :type Boolean)))

(fn GetAttackMontage
  (return 0))

(fn GetAvatar
  (return 0))

(fn GetBloodEffect
  (return 0))

(fn GetCharacterClass
  (return "Elementalist"))

(fn GetCombatSocketLocation
  (params (MontageTag :type Gameplay%20Tag%20Structure%20%28by%20ref%29))
  (return "0, 0, 0"))

(fn GetHitReactMontage
  (return 0))

(fn GetMinionCount
  (return 0))

(fn GetPlayerLevel
  (return 0))

(fn GetTaggedMontagebyTag
  (params (MontageTag :type Gameplay%20Tag%20Structure%20%28by%20ref%29))
  (return ""))

(fn GetWeapon
  (return 0))

(fn IsBeingShocked
  (return false))

(fn IsDead
  (return false))