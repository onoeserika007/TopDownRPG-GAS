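; GA_Firebolt is a gameplay ability that casts a Firebolt projectile toward the location under the mouse.
; On activation it obtains target data, turns the avatar toward the hit point through CombatInterface, draws a debug sphere and plays the cast montage.
; The montage's gameplay event triggers the projectile spawn, and the ability ends after a short delay.
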(event Ability|EventActivateAbility
  (bind _datahandle (|TargetDataUnderMouse)
    (:ValidData
      (Variables|Default|SetTargetLocation (.Location (Collision|BreakHitResult (Ability|TargetData|GetHitResultfromTargetData _datahandle))))
      (bind _ascombat_interface (Utilities|Casting|CastToCombatInterface (Ability|GetAvatarActorfromActorInfo)))
      (Class|CombatInterface|SetFacingTarget _ascombat_interface (Variables|Default|GetTargetLocation))
      (Rendering|Debug|DrawDebugSphere (Variables|Default|GetTargetLocation) 2e+01 12 "(R=1.000000,G=0.968198,B=0.000000,A=1.000000)" 15.0)
      (|PlayMontageandWaitProxy "None" "/Game/Blueprints/Characterr/Aura/Cast_FireBolt_Montage.Cast_FireBolt_Montage" 1.0 "None" true 1.0 0.0
        (:then
          (Ability|Tasks|WaitGameplayEvent "(TagName=\"Event.Montage.FireBolt\")" 0
            (:EventReceived
              (Class|AuraProjectileSpell|SpawnProjectile (Variables|Default|GetTargetLocation))
              (Utilities|FlowControl|Delay 0.5)
              (Ability|EndAbility))))))))

(event Ability|EventOnEndAbility
  (params (bWasCancelled :type Boolean)))

(fn GetHitReactMontage
  (return 0))