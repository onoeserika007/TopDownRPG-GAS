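; Enemy gameplay ability that plays a hit reaction on its avatar.
; On activation it applies GE_HitReact, which carries the tag, and stores the handle, then plays the montage supplied by the avatar's CombatInterface.
; The ability ends when the montage completes, is interrupted or cancelled, or after a fixed delay fallback.
; Ending the ability removes the effect through the stored handle.
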(event Ability|EventActivateAbility
  ;[1 1 1] The GE carries the Tag!!!
  (bind _returnvalue (Ability|ApplyGameplayEffectToOwner "/Game/Blueprints/AbilitySystem/GameplayEffects/GE_HitReact.GE_HitReact_C"))
  (Variables|Default|SetActive%20GE_HitReact _returnvalue)
  (bind _ascombat_interface (Utilities|Casting|CastToCombatInterface (Ability|GetAvatarActorfromActorInfo)))
  (bind _returnvalue_2 (Class|CombatInterface|GetHitReactMontage _ascombat_interface))
  (|PlayMontageandWaitProxy "None" _returnvalue_2 1.0 "None" true 1.0 0.0
    (:then
      (Utilities|FlowControl|Delay 5.0)
      (Ability|EndAbility))
    (:OnCompleted
      (Ability|EndAbility :!label _label))
    (:OnInterrupted
      (goto _label))
    (:OnCancelled
      (goto _label))))

(event Ability|EventOnEndAbility
  (params (bWasCancelled :type Boolean))
  (Ability|RemoveGameplayEffectFromOwnerWithHandle (Variables|Default|GetActive%20GE_HitReact)))