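; Enemy gameplay ability in which a summoner, using a Shaman montage, faces its combat target and summons random minions.
; On the montage's gameplay event, it shuffles the spawn locations and plays a ground effect at each.
; After a short delay, a Delay-driven loop spawns AI-controlled minions one by one, facing away from the summoner, then ends the ability.
; Interface messages raise the summoner's minion count on spawn and lower it on destruction.
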(event Custom|On%20Minion%20Destroyed
  (params (DestroyedActor :type Actor%20Object%20Reference))
  (Class|CombatInterface|IncrementMinionCount(Message) (Ability|GetAvatarActorfromActorInfo) -1))

(event Ability|EventActivateAbility
  (Variables|Default|SetSpawnLocationIndex 0)
  (bind _returnvalue (Class|EnemyInterface|GetCombatTarget(Message) (Ability|GetAvatarActorfromActorInfo)))
  (Variables|Default|SetTargetLocation (Transformation|GetActorLocation _returnvalue))
  (Class|CombatInterface|SetFacingTarget(Message) (Ability|GetAvatarActorfromActorInfo) (Variables|Default|GetTargetLocation))
  (|PlayMontageandWaitProxy "None" "/Game/Blueprints/Character/Shaman/AM_Shaman_Summon.AM_Shaman_Summon" 1.0 "None" true 1.0 0.0
    (:then
      (Ability|Tasks|WaitGameplayEvent "(TagName=\"Montage.Attack.2\")" 0
        (:EventReceived
          (bind _returnvalue_2 (Class|AuraSummonAbility|GetSpawnLocations))
          (bind _output_get (Variables|Default|SetSpawnLocations _returnvalue_2))
          (Utilities|Array|Shuffle _output_get)
          (bind _array_element (Utilities|Array|ForEachLoopwithBreak (Variables|Default|GetSpawnLocations))
            (:LoopBody
              (Niagara|SpawnSystematLocation "/Game/Assets/Effects/Combat/NS_GroundSummon.NS_GroundSummon" _array_element)
              (Utilities|FlowControl|Delay 0.75)
              (if (< (Variables|Default|GetSpawnLocationIndex) (Utilities|Array|Length (Variables|Default|GetSpawnLocations))) :!label _label
                (bind _returnvalue_3 (Game|SpawnActorfromClass (Class|AuraSummonAbility|GetRandomMinionClass) (Math|Transform|MakeTransform (+ (Utilities|Array|Get(acopy) (Variables|Default|GetSpawnLocations) (Variables|Default|GetSpawnLocationIndex)) 7e+01) (Math|Rotator|FindLookatRotation (Math|Conversions|ToVector(Vector2D) (Math|Conversions|ToVector2D(Vector) (Transformation|GetActorLocation (Ability|GetAvatarActorfromActorInfo)))) (Math|Conversions|ToVector(Vector2D) (Math|Conversions|ToVector2D(Vector) (Utilities|Array|Get(acopy) (Variables|Default|GetSpawnLocations) (Variables|Default|GetSpawnLocationIndex))))) "1.000000,1.000000,1.000000") "AdjustIfPossibleButAlwaysSpawn" "MultiplyWithRoot" 0 0))
                (Pawn|SpawnDefaultController _returnvalue_3)
                (Game|BindEventtoOnDestroyed _returnvalue_3 (delegate Custom|On%20Minion%20Destroyed))
                (Class|CombatInterface|IncrementMinionCount(Message) (Ability|GetAvatarActorfromActorInfo) 1)
                (Math|Integer|IncrementInt (Variables|Default|GetSpawnLocationIndex)
                  (:%20%20
                    (Utilities|FlowControl|Delay 0.15)
                    (goto _label)))
                (else
                  (Ability|EndAbility))))))))
    (:OnInterrupted
      (Ability|EndAbility :!label _label_2))
    (:OnCancelled
      (goto _label_2))))

(event Ability|EventOnEndAbility
  (params (bWasCancelled :type Boolean)))