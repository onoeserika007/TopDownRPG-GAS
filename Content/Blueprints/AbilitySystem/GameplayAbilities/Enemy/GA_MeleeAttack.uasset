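; Enemy melee attack ability that faces the avatar toward its combat target and plays a random tagged attack montage.
; The montage's gameplay event triggers a small sphere query at the matching combat socket, damaging non-friendly live players and drawing debug spheres.
; A successful hit executes the MeleeImpact gameplay cue, passing the montage tag so the cue can tell attacks apart.
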(event Ability|EventActivateAbility
  (bind _returnvalue (Ability|GetAvatarActorfromActorInfo))
  (bind _returnvalue_2 (Ability|GetAvatarActorfromActorInfo))
  (bind _returnvalue_3 (Ability|GetAvatarActorfromActorInfo))
  (Variables|Default|SetHasHitTarget false)
  (bind _returnvalue_4 (Class|EnemyInterface|GetCombatTarget(Message) _returnvalue))
  (Utilities|IsValid _returnvalue_4
    (:Is%20Valid
      (Class|CombatInterface|SetFacingTarget(Message) _returnvalue (Transformation|GetActorLocation _returnvalue_4))
      (bind _returnvalue_5 (Class|CombatInterface|GetAttackMontage(Message) _returnvalue))
      (if (> (Utilities|Array|Length _returnvalue_5) 0)
        (Variables|Default|SetLocalTaggedMontage (Utilities|Array|Get(acopy) _returnvalue_5 (Math|Random|RandomIntegerinRange 0 (- (Utilities|Array|Length _returnvalue_5) 1))))
        (|PlayMontageandWaitProxy "None" (.Montage (Utilities|Struct|BreakTaggedMontage (Variables|Default|GetLocalTaggedMontage))) 1.0 "None" true 1.0 0.0
          (:then
            (Ability|Tasks|WaitGameplayEvent (.MontageTag (Utilities|Struct|BreakTaggedMontage (Variables|Default|GetLocalTaggedMontage))) 0
              (:EventReceived
                (bind _returnvalue_6 (Class|CombatInterface|GetCombatSocketLocation(Message) _returnvalue (.SocketTag (Utilities|Struct|BreakTaggedMontage (Variables|Default|GetLocalTaggedMontage)))))
                (bind _output_get (Variables|Default|SetCombatSocketLocation _returnvalue_6))
                (Rendering|Debug|DrawDebugSphere _output_get 45.0 12 "(R=1.000000,G=0.818987,B=0.000000,A=1.000000)" 5.0)
                (bind _outoverlappingactors (Class|AuraAbilitySystemLibrary|GetLivePlayersWithinRadius _returnvalue_2 (Utilities|Array|MakeArray _returnvalue_2) 45.0 (Variables|Default|GetCombatSocketLocation)))
                (for _array_element _outoverlappingactors
                  (Rendering|Debug|DrawDebugSphere (Transformation|GetActorLocation _array_element) 12.0 12 "(R=1.000000,G=0.000000,B=0.043874,A=1.000000)" 5.0)
                  (if (not (Class|AuraAbilitySystemLibrary|IsFriend _array_element (Ability|GetAvatarActorfromActorInfo)))
                    (Class|AuraDamageGameplayAbility|CauseDamage _array_element)
                    (Variables|Default|SetHasHitTarget true)))
                (if (Variables|Default|GetHasHitTarget)
                  (bind _returnvalue_7 (Class|EnemyInterface|GetCombatTarget(Message) _returnvalue_3))
                  (Class|GameplayAbility|ExecuteGameplayCuewithParams "(TagName=\"GameplayCue.MeleeImpact\")" (Ability|GameplayCue|MakeGameplayCueParameters :AggregatedSourceTags (GameplayTags|MakeGameplayTagContainerfromTag (.MontageTag (Utilities|Struct|BreakTaggedMontage (Variables|Default|GetLocalTaggedMontage)))) :Location (Variables|Default|GetCombatSocketLocation) :EffectCauser _returnvalue_3 :SourceObject _returnvalue_7)))
                (Ability|EndAbility))))
          (:OnCompleted
            (Ability|EndAbility :!label _label))
          (:OnInterrupted
            (goto _label))
          (:OnCancelled
            (goto _label)))
        (else
          (Ability|EndAbility))))))

(event Ability|EventOnEndAbility
  (params (bWasCancelled :type Boolean)))