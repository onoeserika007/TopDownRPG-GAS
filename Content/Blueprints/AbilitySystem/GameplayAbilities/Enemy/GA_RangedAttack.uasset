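; Enemy ranged attack gameplay ability that fires a projectile at the avatar's combat target.
; On activation it faces the avatar toward the target's location, then plays a random tagged montage from the avatar's attack list.
; The montage's gameplay event spawns the projectile from its socket tag toward that saved location, prints a debug count and ends the ability.
; Montage completion, interruption, cancellation or an empty list also ends it.
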(event Ability|EventActivateAbility
  (bind _returnvalue (Ability|GetAvatarActorfromActorInfo))
  (bind _returnvalue_2 (Class|EnemyInterface|GetCombatTarget(Message) (Ability|GetAvatarActorfromActorInfo)))
  (Variables|Default|SetTargetLocation (Transformation|GetActorLocation _returnvalue_2))
  (Class|CombatInterface|SetFacingTarget(Message) _returnvalue (Variables|Default|GetTargetLocation))
  (bind _returnvalue_3 (Class|CombatInterface|GetAttackMontage(Message) _returnvalue))
  (if (> (Utilities|Array|Length _returnvalue_3) 0)
    (bind _output_get (Variables|Default|SetLocalTaggedMontage (Utilities|Array|Get(acopy) _returnvalue_3 (Math|Random|RandomIntegerinRange 0 (- (Utilities|Array|Length _returnvalue_3) 1)))))
    (|PlayMontageandWaitProxy "None" (.Montage (Utilities|Struct|BreakTaggedMontage _output_get)) 1.0 "None" true 1.0 0.0
      (:then
        (Ability|Tasks|WaitGameplayEvent (.MontageTag (Utilities|Struct|BreakTaggedMontage _output_get)) 0
          (:EventReceived
            (Class|AuraProjectileSpell|SpawnProjectile (Variables|Default|GetTargetLocation) (.SocketTag (Utilities|Struct|BreakTaggedMontage _output_get)) false 0.0)
            (bind _result (Math|Integer|IncrementInt (Variables|Default|GetCount))
              (:%20%20
                (Development|PrintString (Utilities|String|Append "Projectile Spawned " (Utilities|String|ToString(Integer) _result) " times."))
                ;[1 1 1 1 15] 由于未知原因导致PlayMontage未正常退出时，有可能导致未End Ability导致多份Instance。未正常退出Montage播放的情况不是yin jiao li de ren he yi zhong.
                (Ability|EndAbility))))))
      (:OnCompleted
        (Ability|EndAbility :!label _label))
      (:OnInterrupted
        (goto _label))
      (:OnCancelled
        (goto _label)))
    (else
      (Ability|EndAbility))))

(event Ability|EventOnEndAbility
  (params (bWasCancelled :type Boolean)))