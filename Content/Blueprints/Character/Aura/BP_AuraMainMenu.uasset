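; BP_AuraMainMenu is the main menu scene actor for Aura, animating the display and launching the menu UI.
; On BeginPlay it starts the menu music, adds WBP_MainMenu to the viewport, and switches to UI-only input with a visible cursor.
; Tick accumulates time to bob the Fire component vertically on a sine wave around its initial location and steadily rolls the magic circle decal.
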(event EventBeginPlay
  (bind _returnvalue (Game|GetPlayerController 0))
  (Variables|Default|SetFireInitLoc (Transformation|GetWorldLocation (Variables|Default|GetFire)))
  (Audio|PlaySound2D "/Game/Assets/Sounds/Music/Music_MainMenu.Music_MainMenu" 1.0 1.0 0.0 0 0)
  (bind _returnvalue_2 (UserInterface|CreateWidget "/Game/Blueprints/UI/MainMenu/WBP_MainMenu.WBP_MainMenu_C" (Game|GetPlayerController 0)))
  (UserInterface|Viewport|AddtoViewport _returnvalue_2 0)
  (Input|SetInputModeUIOnly _returnvalue 0 "DoNotLock" false)
  (Variables|/Script/Engine.PlayerController|SetbShowMouseCursor _returnvalue true))

(event Collision|EventActorBeginOverlap
  (params (OtherActor :type Actor%20Object%20Reference)))

(event EventTick
  (params (DeltaSeconds :type Float%20%28single-precision%29))
  (bind _output_get (Variables|Default|SetDeltaSeconds DeltaSeconds))
  (Variables|Default|SetTime (+ _output_get (Variables|Default|GetTime)))
  (Utilities|FlowControl|Sequence
    (:then_0
      (Transformation|SetWorldLocation (Variables|Default|GetFire) (+ (* (Math|Trig|Sin(Radians) (* (Variables|Default|GetTime) (Variables|Default|GetFireShakeFrequency))) "0.000000,0.000000,3.000000") (Variables|Default|GetFireInitLoc)) false false))
    (:then_1
      (Transformation|AddLocalRotation (Variables|Default|GetMagicCircleDecal) (Math|Rotator|MakeRotator (* (Variables|Default|GetDeltaSeconds) 2e+01) 0.0 0.0) false false))))

(fn ConstructionScript)