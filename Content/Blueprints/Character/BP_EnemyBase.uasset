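; Base Blueprint for enemy characters, providing their spawn and dissolve visuals plus attack-facing support through motion warping.
; On BeginPlay a timeline drives uniform actor scale for the spawn effect.
; Two dissolve events run separate timelines that animate the Dissolve parameter on supplied dynamic materials, one of them for the weapon.
; SetFacingTarget updates the FacingTarget warp target location on the MotionWarping component.
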(event EventBeginPlay
  (bind _spawn (Timeline|SpawnTimeline Play)
    (:Update
      (Transformation|SetActorRelativeScale3D (Math|Vector|MakeVector _spawn _spawn _spawn)))))

(event Collision|EventActorBeginOverlap
  (params (OtherActor :type Actor%20Object%20Reference)))

(event EventTick
  (params (DeltaSeconds :type Float%20%28single-precision%29)))

(event EventStartDissolveTimeline
  (params (DynamicMaterialInstance :type Material%20Instance%20Dynamic%20Object%20Reference))
  (bind _dissolvetrack (Timeline|时间轴 Play)
    (:Update
      (Rendering|Material|SetScalarParameterValue DynamicMaterialInstance "Dissolve" _dissolvetrack :!class /Script/Engine.MaterialInstanceDynamic))))

(event EventStartWeaponDissolveTimeline
  (params (DynamicMaterialInstance :type Material%20Instance%20Dynamic%20Object%20Reference))
  (bind _dissolvetrack (Timeline|时间轴_0 Play)
    (:Update
      (Rendering|Material|SetScalarParameterValue DynamicMaterialInstance "Dissolve" _dissolvetrack :!class /Script/Engine.MaterialInstanceDynamic))))

(event EventSetFacingTarget
  (params (FacingTarget :type Vector%20%28by%20ref%29 :default "0, 0, 0"))
  (Class|MotionWarpingComponent|AddorUpdateWarpTargetfromLocation (Variables|Default|GetMotionWarping) "FacingTarget" FacingTarget))

(fn ConstructionScript)